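; Player character with smoothed mouse-look panning and automated walking to target actors.
; OrientMovement levels control pitch with a timeline, then switches rotation to follow movement and starts SimpleMoveToLocation toward the target.
; While moving, Tick asks the player controller for a distance check; on arrival ReturnToPlayerStatus stops movement, aligns actor and control rotation to the camera yaw, resets rotation flags and walk speed, and re-enables click/tap.
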(event Custom|Return%20to%20Player%20Status
  (bind _as_bp_my_player_controller (Variables|Default|GetAs%20Bp%20My%20Player%20Controller))
  (Utilities|FlowControl|Sequence
    (:then_0
      (Variables|Default|SetZ%20Rotation%20Mov (.yaw (Transformation|GetActorRotation (Variables|Default|GetLocation%20Target)))))
    (:then_1
      (Variables|Default|SetLocation%20Target (Variables|Default|GetLocationFalse)))
    (:then_2
      (Variables|Default|SetReturn%20Value%20Z%20%28Yaw%29 (.yaw (Transformation|GetWorldRotation (Variables|Default|GetCameraMyPlayer)))))
    (:then_3
      (AI|Navigation|StopMovement _as_bp_my_player_controller)
      (Transformation|SetActorRotation (Math|Rotator|MakeRotator 0.0 0.0 (Variables|Default|GetReturn%20Value%20Z%20%28Yaw%29)))
      (Pawn|SetControlRotation _as_bp_my_player_controller (Math|Rotator|MakeRotator 0.0 0.0 (Variables|Default|GetReturn%20Value%20Z%20%28Yaw%29)))
      (Variables|Default|SetStart%20Movement false)
      (CallFunction|ToOrient true false true false)
      (Variables|/Game/Blueprint/Gamemode/Bp_MyPlayerController.Bp_MyPlayerController_C|SetCan%20Click/Tap (Variables|Default|GetAs%20Bp%20My%20Player%20Controller) true)
      (Variables|/Script/Engine.CharacterMovementComponent|SetMaxWalkSpeed (Variables|Character|GetCharacterMovement) 1e+02))
    (:then_4
      (Development|PrintString "Return to Player Status"))))

(event Custom|Orient%20Movement
  (params (TargetLocation :type Target%20Point%20Object%20Reference))
  (Variables|Default|SetLocation%20Target TargetLocation)
  (Utilities|FlowControl|Sequence
    (:then_0
      (Variables|Default|SetReturn%20Value%20Y%20%28Pitch%29_0 (.pitch (Transformation|GetWorldRotation (Variables|Default|GetCameraMyPlayer))))
      (Variables|Default|SetReturn%20Value%20Z%20%28Yaw%29 (.yaw (Pawn|GetControlRotation (Variables|Default|GetAs%20Bp%20My%20Player%20Controller) :!class /Script/Engine.Controller))))
    (:then_1
      (bind _newtrack_0 (Timeline|Timeline_1 PlayFromStart)
        (:Update
          (Pawn|SetControlRotation (Variables|Default|GetAs%20Bp%20My%20Player%20Controller) (Math|Rotator|MakeRotator 0.0 (Math|Float|Lerp (Variables|Default|GetReturn%20Value%20Y%20%28Pitch%29_0) 0.0 _newtrack_0) (Variables|Default|GetReturn%20Value%20Z%20%28Yaw%29))))
        (:Finished
          (Variables|Default|SetStart%20Movement true)
          (AI|Navigation|SimpleMovetoLocation (Variables|Default|GetAs%20Bp%20My%20Player%20Controller) (Transformation|GetActorLocation (Variables|Default|GetLocation%20Target)))
          (CallFunction|ToOrient false true false true))))))

(event EventBeginPlay
  (Utilities|FlowControl|Sequence
    (:then_0
      (CallFunction|SetPlayerMove true))
    (:then_1
      (bind _asbp_my_player_controller (Utilities|Casting|CastToBp_MyPlayerController (Game|GetPlayerController 0)))
      (Variables|Default|SetAs%20Bp%20My%20Player%20Controller _asbp_my_player_controller))))

(event EventTick
  (params (DeltaSeconds :type Float%20%28single-precision%29))
  (if (Variables|Default|GetStart%20Movement)
    (if (Default|CheckTargetDistance (Variables|Default|GetAs%20Bp%20My%20Player%20Controller) (Variables|Default|GetLocation%20Target) 75.0)
      (CallFunction|ReturntoPlayerStatus)
      (else
        (Development|PrintString "far")))
    (else
      (Development|PrintString "no movement"))))

(event Input|MouseEvents|MouseY
  (params (AxisValue :type Float%20%28single-precision%29))
  ;[0 0 0] Pan Character
  (if (Variables|Default|GetCanPanCharacter)
    (bind _output_get (Variables|Default|SetCurrentYMouse (Math|Interpolation|FInterpTo (Variables|Default|GetCurrentYMouse) (* (Variables|Default|GetPanSpeedCharacter) AxisValue) (Utilities|Time|GetWorldDeltaSeconds) 5.0)))
    (Pawn|Input|AddControllerPitchInput _output_get)))

(event Input|MouseEvents|MouseX
  (params (AxisValue :type Float%20%28single-precision%29))
  ;[0 0 0] Pan Character
  (if (Variables|Default|GetCanPanCharacter)
    (bind _output_get (Variables|Default|SetCurrentXMouse (Math|Interpolation|FInterpTo (Variables|Default|GetCurrentXMouse) (* AxisValue (* -1.0 (Variables|Default|GetPanSpeedCharacter))) (Utilities|Time|GetWorldDeltaSeconds) 5.0)))
    (Pawn|Input|AddControllerYawInput _output_get)))

(fn ConstructionScript)

(fn ToOrient
  (params (Use%20Controller%20Rotation%20Yaw :type Boolean) (Use%20Controller%20Rotation%20Pitch :type Boolean) (Use%20Pawn%20Control%20Rotation :type Boolean) (Orient%20Rotation%20to%20Movement :type Boolean))
  (Utilities|FlowControl|Sequence
    (:then_0
      (Variables|Default|SetbUseControllerRotationYaw Use%20Controller%20Rotation%20Yaw))
    (:then_1
      (Variables|Default|SetbUseControllerRotationPitch Use%20Controller%20Rotation%20Pitch))
    (:then_2
      (Variables|/Script/Engine.CameraComponent|SetbUsePawnControlRotation (Variables|Default|GetCameraMyPlayer) Use%20Pawn%20Control%20Rotation))
    (:then_3
      (Variables|/Script/Engine.CharacterMovementComponent|SetbOrientRotationToMovement (Variables|Character|GetCharacterMovement) Orient%20Rotation%20to%20Movement))
    (:then_4
      (return))))

(fn SetPlayerMove
  (params (CanPanCharacter :type Boolean))
  (Variables|Default|SetCanPanCharacter CanPanCharacter)
  (return))