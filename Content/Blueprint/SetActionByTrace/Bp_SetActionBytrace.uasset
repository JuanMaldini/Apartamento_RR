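; Configurable interactable actor that toggles between start and back states when its action event fires, briefly flashing an icon outline.
; Boolean options select each effect: camera blend, icon hiding, fridge popup, cinema widget, media with sound, light and material changes, and forward or reversed level sequences.
; `CanPass` and `IsInStartEvent` gate the toggle, and light intensity is set by a one-shot Lerp.
; A separate function switches living-room and bedroom TVs.
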(event OnComponentBeginOverlap(BoxFalse)
  (params (OverlappedComponent :type Primitive%20Component%20Object%20Reference) (OtherActor :type Actor%20Object%20Reference) (OtherComp :type Primitive%20Component%20Object%20Reference) (OtherBodyIndex :type Integer) (bFromSweep :type Boolean) (SweepResult :type Hit%20Result%20Structure%20%28by%20ref%29))
  (Rendering|SetVisibility (Variables|Default|GetBoxFalse) false false))

(event Custom|BP-Action
  ;[0 0 0] Make Action
  (Utilities|FlowControl|Sequence
    (:then_0
      (Utilities|SetOutlineTimer))
    (:then_1
      (switch Utilities|FlowControl|Switch|SwitchonAction_Enum (Variables|Modificable|GetAction)
        (:NewEnumerator2
          (if (Variables|GenericBlueprint|GetIs%20in%20StartEvent)
            (CallFunction|BackfromStartAction)
            (else
              (CallFunction|StartAction))))))))

(event Custom|BP-BackFromAction
  ;[0 0 0] Go to Start Action
  ;[0 0 0] Back from Start Action
  (CallFunction|BackfromStartAction))

(event Custom|Back%20from%20Start%20Action
  (bind _blend_time (Variables|GenericBlueprint|GetBlend%20Time))
  (bind _light___intensity_off (Variables|Modificable|GetLight%20-%20Intensity%20Off))
  (bind _light___intensity_on (Variables|Modificable|GetLight%20-%20Intensity%20On))
  (bind _returnvalue (Math|Float|Lerp _light___intensity_off _light___intensity_on _blend_time))
  ;[0 0 0] Back from Start Action
  (if (Variables|GenericBlueprint|GetIs%20in%20StartEvent)
    (if (Variables|GenericBlueprint|GetCan%20pass)
      (Variables|GenericBlueprint|SetCan%20pass false)
      (Utilities|FlowControl|Sequence
        (:then_0
          (if (Variables|Modificable|GetBlend%20-%20Camera)
            (Game|Player|SetViewTargetwithBlend (Game|GetPlayerController 0) (Variables|GenericBlueprint|GetAs%20Bp%20My%20Player%20Characer) (Variables|GenericBlueprint|GetBlend%20Time) "VTBlend_Linear" 0.0 false)
            (bind _asbp_my_player_controller (Utilities|Casting|CastToBp_MyPlayerController (Game|GetPlayerController 0)))
            (Variables|/Game/Blueprint/Gamemode/Bp_MyPlayerController.Bp_MyPlayerController_C|SetCan%20Click/Tap _asbp_my_player_controller true)))
        (:then_1
          (if (Variables|Modificable|GetIcon%20-%20Hide%20in%20Interact)
            (Rendering|SetVisibility (Variables|Default|GetIcon) true true)))
        (:then_2
          (if (Variables|Modificable|GetCine)
            (Widget|RemovefromParent (Variables|Default|GetBackCineRef))))
        (:then_3
          (if (Variables|Modificable|GetMedia%202D)
            (Rendering|Material|SetMaterial (Variables|/Script/Engine.StaticMeshActor|GetStaticMeshComponent (Variables|Modificable|GetTv%20-%20Cine)) 0 0)
            (Audio|Components|Audio|Stop (Variables|Default|GetCine%20Sound))))
        (:then_4
          (if (Variables|Modificable|GetLight)
            (Utilities|FlowControl|Sequence
              (:then_0
                (for _array_element (Variables|Modificable|GetLight%20-%20Spot)
                  (Rendering|Components|Light|SetIntensity (Variables|/Script/Engine.SpotLight|GetSpotLightComponent _array_element) _returnvalue)))
              (:then_1
                (for _array_element_2 (Variables|Modificable|GetLight%20-%20Point)
                  (Rendering|Components|Light|SetIntensity (Variables|/Script/Engine.Light|GetLightComponent _array_element_2) _returnvalue)))
              (:then_2
                (if (Variables|Modificable|GetLight%20-%20Set%20Material%20in%20Spot)
                  (for _array_element_3 (Variables|Modificable|GetLight%20-%20Metallic%20Spot)
                    (Rendering|Material|SetMaterial (Variables|/Script/Engine.StaticMeshActor|GetStaticMeshComponent _array_element_3) 1 0)))))))
        (:then_5
          (if (Variables|Modificable|GetSequence%20A)
            (if (Variables|Modificable|GetInvert%20Sequence%20A)
              (bind _returnvalue_2 (Sequencer|Player|CreateLevelSequencePlayer (Variables|Modificable|GetSequence%20A%20-%20Ref)))
              (Sequencer|Player|Play _returnvalue_2 :!class /Script/MovieScene.MovieSceneSequencePlayer)
              (else
                (bind _returnvalue_3 (Sequencer|Player|CreateLevelSequencePlayer (Variables|Modificable|GetSequence%20A%20-%20Ref)))
                (Class|MovieSceneSequencePlayer|PlayReverse _returnvalue_3)))))
        (:then_6
          (if (Variables|Modificable|GetSequence%20B)
            (bind _returnvalue_4 (Sequencer|Player|CreateLevelSequencePlayer (Variables|Modificable|GetSequence%20B%20-%20Ref)))
            (Class|MovieSceneSequencePlayer|PlayReverse _returnvalue_4)))
        (:then_7
          (if (Variables|Modificable|GetSequence%20A)
            (Utilities|FlowControl|Delay (Variables|Modificable|GetTime%20-%20Enable%20Back)))
          (Variables|GenericBlueprint|SetCan%20pass true)
          (Variables|GenericBlueprint|SetIs%20in%20StartEvent false))))))

(event Custom|Start%20Action
  (bind _light___intensity_off (Variables|Modificable|GetLight%20-%20Intensity%20Off))
  (bind _blend_time (Variables|GenericBlueprint|GetBlend%20Time))
  (bind _light___intensity_on (Variables|Modificable|GetLight%20-%20Intensity%20On))
  (bind _sequence_a___ref (Variables|Modificable|GetSequence%20A%20-%20Ref))
  (bind _returnvalue (Math|Float|Lerp _light___intensity_on _light___intensity_off _blend_time))
  ;[0 0 0] Go to Start Action
  (if (Variables|GenericBlueprint|GetCan%20pass)
    (Variables|GenericBlueprint|SetCan%20pass false)
    (Utilities|FlowControl|Sequence
      (:then_0
        (if (Variables|Modificable|GetBlend%20-%20Camera)
          (Game|Player|SetViewTargetwithBlend (Game|GetPlayerController 0) (Variables|Modificable|GetBlend%20-%20Camera%20Ref) (Variables|GenericBlueprint|GetBlend%20Time) "VTBlend_Linear" 0.0 false)
          (Utilities|FlowControl|Sequence
            (:then_0
              (bind _asbp_my_game_mode_level_a (Utilities|Casting|CastToBp_MyGameMode_Level_A (Game|GetGameMode)))
              (Widget|RemovefromParent (Variables|/Game/Blueprint/Gamemode/Bp_MyGameMode_Level_A.Bp_MyGameMode_Level_A_C|GetW_DefaultScreenFull_Ref _asbp_my_game_mode_level_a)))
            (:then_1
              (bind _asbp_my_player_controller (Utilities|Casting|CastToBp_MyPlayerController (Game|GetPlayerController 0)))
              (Variables|/Game/Blueprint/Gamemode/Bp_MyPlayerController.Bp_MyPlayerController_C|SetCan%20Click/Tap _asbp_my_player_controller false)))))
      (:then_1
        (if (Variables|Modificable|GetIcon%20-%20Hide%20in%20Interact)
          (Rendering|SetVisibility (Variables|Default|GetIcon) false false)))
      (:then_2
        (if (Variables|Modificable|GetFrigo)
          (bind _asbp_my_game_mode_level_a_2 (Utilities|Casting|CastToBp_MyGameMode_Level_A (Game|GetGameMode)))
          (UserInterface|Viewport|AddtoViewport (Variables|/Game/Blueprint/Gamemode/Bp_MyGameMode_Level_A.Bp_MyGameMode_Level_A_C|GetW_Pop-up_Frigo_Ref _asbp_my_game_mode_level_a_2) 0)))
      (:then_3
        (if (Variables|Modificable|GetCine)
          (bind _returnvalue_2 (UserInterface|CreateWidget "/Game/Blueprint/Menu/W_BackCine.W_BackCine_C"))
          (bind _output_get (Variables|Default|SetBackCineRef _returnvalue_2))
          (UserInterface|Viewport|AddtoViewport _output_get 0)))
      (:then_4
        (if (Variables|Modificable|GetMedia%202D)
          (Utilities|FlowControl|Delay (Variables|Modificable|GetTime%20-%20Enable%20Back))
          (Media|MediaPlayer|OpenSource (Variables|GenericBlueprint|GetMedia%20Player%2002) (Variables|GenericBlueprint|GetMedia%20Source%2002))
          (Rendering|Material|SetMaterial (Variables|/Script/Engine.StaticMeshActor|GetStaticMeshComponent (Variables|Modificable|GetTv%20-%20Cine)) 0 0)
          (bind _returnvalue_3 (Audio|SpawnSound2D 0 1.0 1.0 0.0 0))
          (Variables|Default|SetCine%20Sound _returnvalue_3)))
      (:then_5
        (if (Variables|Modificable|GetLight)
          (Utilities|FlowControl|Sequence
            (:then_0
              (for _array_element (Variables|Modificable|GetLight%20-%20Spot)
                (Rendering|Components|Light|SetIntensity (Variables|/Script/Engine.SpotLight|GetSpotLightComponent _array_element) _returnvalue)))
            (:then_1
              (for _array_element_2 (Variables|Modificable|GetLight%20-%20Point)
                (Rendering|Components|Light|SetIntensity (Variables|/Script/Engine.Light|GetLightComponent _array_element_2) _returnvalue)))
            (:then_2
              (if (Variables|Modificable|GetLight%20-%20Set%20Material%20in%20Spot)
                (for _array_element_3 (Variables|Modificable|GetLight%20-%20Metallic%20Spot)
                  (Rendering|Material|SetMaterial (Variables|/Script/Engine.StaticMeshActor|GetStaticMeshComponent _array_element_3) 1 0)))))))
      (:then_6
        (if (Variables|Modificable|GetSequence%20A)
          (if (Variables|Modificable|GetInvert%20Sequence%20A)
            (bind _returnvalue_4 (Sequencer|Player|CreateLevelSequencePlayer _sequence_a___ref))
            (Class|MovieSceneSequencePlayer|PlayReverse _returnvalue_4)
            (else
              (bind _returnvalue_5 (Sequencer|Player|CreateLevelSequencePlayer _sequence_a___ref))
              (Sequencer|Player|Play _returnvalue_5 :!class /Script/MovieScene.MovieSceneSequencePlayer)))))
      (:then_7
        (if (Variables|Modificable|GetSequence%20B)
          (bind _returnvalue_6 (Sequencer|Player|CreateLevelSequencePlayer (Variables|Modificable|GetSequence%20B%20-%20Ref)))
          (Sequencer|Player|Play _returnvalue_6 :!class /Script/MovieScene.MovieSceneSequencePlayer)))
      (:then_8
        (if (Variables|Modificable|GetSequence%20A)
          (Utilities|FlowControl|Delay (Variables|Modificable|GetTime%20-%20Enable%20Back)))
        (Variables|GenericBlueprint|SetCan%20pass true)
        (Variables|GenericBlueprint|SetIs%20in%20StartEvent true)))))

(event EventBeginPlay
  ;[0 0 0] Begin Play
  (Utilities|FlowControl|Sequence
    (:then_0
      (bind _asbp_my_player_characer_01 (Utilities|Casting|CastToBp_AV_Player (Game|GetPlayerCharacter 0)))
      (Variables|GenericBlueprint|SetAs%20Bp%20My%20Player%20Characer _asbp_my_player_characer_01))
    (:then_1
      (bind _asbp_my_game_mode_level_a (Utilities|Casting|CastToBp_MyGameMode_Level_A (Game|GetGameMode)))
      (Variables|WidgetRef|SetW%20Pop-up%20Frigo%20Ref (Variables|/Game/Blueprint/Gamemode/Bp_MyGameMode_Level_A.Bp_MyGameMode_Level_A_C|GetW_Pop-up_Frigo_Ref _asbp_my_game_mode_level_a)))))

(fn ConstructionScript
  (Rendering|SetVisibility (Variables|Default|GetBoxFalse) (Variables|Default|GetBoxFalseVisible) false))