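; Player character for an architectural visualization walkthrough, handling mouse look and jumps to target viewpoints.
; While the Archvizz controller's CanClick flag is set, mouse axes are scaled, smoothed with FInterpTo and applied as yaw and pitch, with horizontal input inverted.
; OrientMovement stops movement, teleports to the target actor, then uses a timeline to blend control rotation from the prior view to level pitch and the target's yaw.
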(event Custom|Orient%20Movement
  (params (TargetLocation :type Actor%20Object%20Reference))
  (Variables|Default|SetLocation%20Target TargetLocation)
  (AI|Navigation|StopMovement (Variables|Default|GetAs%20Bp%20My%20Player%20Controller))
  (Utilities|FlowControl|Sequence
    (:then_0
      (Variables|Default|SetReturn%20Value%20Y%20%28Pitch%29_0 (.pitch (Transformation|GetWorldRotation (Variables|Default|GetCameraMyPlayer))))
      (Variables|Default|SetReturn%20Value%20Z%20%28Yaw%29 (.yaw (Pawn|GetControlRotation (Variables|Default|GetAs%20Bp%20My%20Player%20Controller) :!class /Script/Engine.Controller))))
    (:then_1
      (Transformation|Teleport (Transformation|GetActorLocation (Variables|Default|GetLocation%20Target)) (Transformation|GetActorRotation (Variables|Default|GetLocation%20Target))))
    (:then_2
      (bind _newtrack_0 (Timeline|Timeline_1 PlayFromStart)
        (:Update
          (Pawn|SetControlRotation (Variables|Default|GetAs%20Bp%20My%20Player%20Controller) (Math|Rotator|MakeRotator 0.0 (Math|Float|Lerp (Variables|Default|GetReturn%20Value%20Y%20%28Pitch%29_0) 0.0 _newtrack_0) (Math|Float|Lerp (Variables|Default|GetReturn%20Value%20Z%20%28Yaw%29) (.yaw (Transformation|GetActorRotation (Variables|Default|GetLocation%20Target))) _newtrack_0))))))))

(event EventBeginPlay
  (bind _asbp_controller_archvizz (Utilities|Casting|CastToBp_Controller_Archvizz (Game|GetPlayerController 0)))
  (Variables|Default|SetAs%20Bp%20My%20Player%20Controller _asbp_controller_archvizz))

(event Input|MouseEvents|MouseY
  (params (AxisValue :type Float%20%28single-precision%29))
  ;[0 0 0] Pan Character
  (if (Variables|/Game/Blueprint/Gamemode/Bp_Controller_Archvizz.Bp_Controller_Archvizz_C|GetCanClick (Variables|Default|GetAs%20Bp%20My%20Player%20Controller))
    (bind _output_get (Variables|Default|SetCurrentYMouse (Math|Interpolation|FInterpTo (Variables|Default|GetCurrentYMouse) (* 0.8 AxisValue) (Utilities|Time|GetWorldDeltaSeconds) 5.0)))
    (Pawn|Input|AddControllerPitchInput _output_get)))

(event Input|MouseEvents|MouseX
  (params (AxisValue :type Float%20%28single-precision%29))
  ;[0 0 0] Pan Character
  (if (Variables|/Game/Blueprint/Gamemode/Bp_Controller_Archvizz.Bp_Controller_Archvizz_C|GetCanClick (Variables|Default|GetAs%20Bp%20My%20Player%20Controller))
    (bind _output_get (Variables|Default|SetCurrentXMouse (Math|Interpolation|FInterpTo (Variables|Default|GetCurrentXMouse) (* AxisValue (* -1.0 0.8)) (Utilities|Time|GetWorldDeltaSeconds) 5.0)))
    (Pawn|Input|AddControllerYawInput _output_get)))

(fn ConstructionScript)