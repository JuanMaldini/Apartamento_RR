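; Floorplan camera pawn or character that orbits and zooms a spring-arm view using mouse input.
; MouseX and MouseY axes feed controller yaw and pitch, with an initial pitch nudge on BeginPlay.
; The MouseX handler also clamps control-rotation pitch to a downward-looking range and zeroes roll.
; Mouse wheel steps the spring arm length within fixed near and far limits.
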(event EventBeginPlay
  (Pawn|Input|AddControllerPitchInput 1e+01))

(event Input|MouseEvents|MouseX
  (params (AxisValue :type Float%20%28single-precision%29))
  (bind _returnvalue (Pawn|GetControlRotation :!class /Script/Engine.Pawn))
  (Pawn|Input|AddControllerYawInput AxisValue)
  (Pawn|SetControlRotation (Game|GetPlayerController 0) (Math|Rotator|MakeRotator 0.0 (Math|Float|ClampAngle (.pitch _returnvalue) 3e+02 3.4e+02) (.yaw _returnvalue))))

(event Input|MouseEvents|MouseY
  (params (AxisValue :type Float%20%28single-precision%29))
  (Pawn|Input|AddControllerPitchInput AxisValue))

(event Input|MouseEvents|MouseWheelUp
  (params (Key :type Key%20Structure :default "None"))
  (bind _springarm (Variables|Default|GetSpringArm))
  (:Pressed
    (Variables|/Script/Engine.SpringArmComponent|SetTargetArmLength _springarm (Math|Float|Clamp(Float) (- (Variables|/Script/Engine.SpringArmComponent|GetTargetArmLength _springarm) 1e+02) 1e+03 2.5e+03))))

(event Input|MouseEvents|MouseWheelDown
  (params (Key :type Key%20Structure :default "None"))
  (bind _springarm (Variables|Default|GetSpringArm))
  (:Pressed
    (Variables|/Script/Engine.SpringArmComponent|SetTargetArmLength _springarm (Math|Float|Clamp(Float) (+ (Variables|/Script/Engine.SpringArmComponent|GetTargetArmLength _springarm) 1e+02) 1e+03 2.5e+03))))

(fn ConstructionScript)