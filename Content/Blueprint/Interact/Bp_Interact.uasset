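; Interactable door controller that toggles a door open or closed when the player's Interact event fires.
; On construction it snaps to the referenced door, stores its yaw and sets two status texts.
; LerpCinematic selects a Level Sequence played forward or reversed, or an Open timeline rotating the controller's tag-matched HitActor, with optional flipped direction.
; Both paths update the open state and text, and briefly outline the hit mesh via custom depth.
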(event Custom|Interact
  (switch Utilities|FlowControl|Switch|SwitchonAction (Variables|01-Generic|GetAction)
    (:NewEnumerator0
      (if (Variables|02-BpDoor|GetLerp%20/%20Cinematic?)
        (|OpenwithCinematic)
        (else
          (|Openwithlerp))))))

(event EventBeginPlay
  (Utilities|FlowControl|Sequence
    (:then_0
      (bind _asbp_av_player (Utilities|Casting|CastToBp_AV_Player (Game|GetPlayerCharacter 0)))
      (Variables|Default|SetAs%20Bp%20AV%20Player _asbp_av_player))
    (:then_1
      (bind _asbp_my_player_controller (Utilities|Casting|CastToBp_MyPlayerController (Game|GetPlayerController 0)))
      (Variables|Default|SetAs%20Bp%20My%20Player%20Controller _asbp_my_player_controller))
    (:then_2
      (Utilities|IsValid (Variables|Default|GetAs%20Bp%20AV%20Player)
        (:Is%20Valid
          ;[0 0 0] E Event
          (EventDispatchers|BindEventtoInteract (Variables|Default|GetAs%20Bp%20AV%20Player) (delegate Custom|Interact)))
        (:Is%20Not%20Valid
          (Actor|DestroyActor))))))

(fn ConstructionScript
  (switch Utilities|FlowControl|Switch|SwitchonAction (Variables|01-Generic|GetAction)
    (:NewEnumerator0
      (|OpenDoor))))

(fn TextStatus
  (params (Value :type Text) (InLinearColor :type Linear%20Color%20Structure))
  (bind _textrender_02 (Variables|Default|GetTextRender_02))
  (Rendering|Components|TextRender|SetText _textrender_02 Value)
  (Rendering|Components|TextRender|SetTextRenderColor _textrender_02 (Class|KismetMathLibrary|LinearColortoRGBE InLinearColor))
  (return))

(event Custom|OnFinished_Event_Forward
  (CallFunction|TextStatus "IS OPEN" "(R=0.000000,G=1.000000,B=0.000000,A=1.000000)")
  (return))

(event Custom|OnFinished_Event_Backguard
  (CallFunction|TextStatus "IS CLOSED" "(R=1.000000,G=0.000000,B=0.000000,A=1.000000)")
  (return))