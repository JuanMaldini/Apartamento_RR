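; Interactable actor for doors, still unfinished: at BeginPlay it binds to the player's interact event, which currently only prints a debug message.
; An Action switch in the construction script drives door setup, snapping the actor to the referenced door and showing open/closed state on two colored text renders.
; An Open Door function toggles IsOpen on the controller's tagged hit actor, but its yaw rotation logic is unwired.
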(event Custom|Interact
  (Development|PrintString "MAKE INTERACT!"))

(event EventBeginPlay
  (Utilities|FlowControl|Sequence
    (:then_0
      (bind _asbp_av_player (Utilities|Casting|CastToBp_AV_Player (Game|GetPlayerCharacter 0)))
      (Variables|Default|SetAs%20Bp%20AV%20Player _asbp_av_player))
    (:then_1
      (bind _asbp_my_player_controller (Utilities|Casting|CastToBp_MyPlayerController (Game|GetPlayerController 0)))
      (Variables|Default|SetAs%20Bp%20My%20Player%20Controller _asbp_my_player_controller))
    (:then_2
      ;[0 0 0] E Event
      (EventDispatchers|BindEventtoInteract (Variables|Default|GetAs%20Bp%20AV%20Player) (delegate Custom|Interact)))))

(fn ConstructionScript
  (switch Utilities|FlowControl|Switch|SwitchonAction (Variables|Default|GetAction)
    (:NewEnumerator0
      (|OpenDoor))))

(fn TextStatus
  (params (Value :type Text) (Color :type Color%20Structure))
  (bind _textrender (Variables|Default|GetTextRender))
  (Rendering|Components|TextRender|SetText _textrender Value)
  (Rendering|Components|TextRender|SetTextRenderColor _textrender Color)
  (return))

(fn OpenDoor
  (bind _as_bp_my_player_controller (Variables|Default|GetAs%20Bp%20My%20Player%20Controller))
  (bind _hit_actor (Variables|/Game/Blueprint/Gamemode/Bp_MyPlayerController.Bp_MyPlayerController_C|GetHit%20Actor _as_bp_my_player_controller))
  (bind _returnvalue (Transformation|GetActorRotation _hit_actor))
  (Utilities|IsValid _hit_actor
    (:Is%20Valid
      (if (Actor|ActorHasTag _hit_actor (Variables|0-BpDoor|GetTag))
        (if (Variables|0-BpDoor|GetIsOpen)
          (Variables|Default|SetOriginal%20Rotation _returnvalue)
          (Variables|0-BpDoor|SetIsOpen false)
          (else
            (Variables|Default|SetOriginal%20Rotation _returnvalue)
            (Variables|0-BpDoor|SetIsOpen true)))
        (else
          (Development|PrintString "no tag"))))
    (:Is%20Not%20Valid
      (Development|PrintString "NO VALID"))))