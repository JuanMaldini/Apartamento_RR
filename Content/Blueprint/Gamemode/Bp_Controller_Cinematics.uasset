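; Player controller for cinematics that shows the mouse cursor and holds click/touch navigation helpers, none called within this graph.
; Helpers trace mouse or touch into the world, path to FLOOR-tagged hits with a target marker, rotate the view by touch, and orient Bp_AV_Player from minimap points.
; A retriggerable-delay macro separates single from double clicks.
; A Pixel Streaming handler runs received strings as console commands, but its binding is disconnected.
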(event Custom|PixelInput
  (params (Descriptor :type String))
  (bind _pixelstreaminginput (Variables|Components|GetPixelStreamingInput))
  (Variables|Default|SetDescriptor Descriptor)
  (if (.Success (Class|PixelStreamingInput|GetJsonStringValue _pixelstreaminginput (Variables|Default|GetDescriptor)))
    (Development|ExecuteConsoleCommand (.StringValue (Class|PixelStreamingInput|GetJsonStringValue _pixelstreaminginput (Variables|Default|GetDescriptor))) 0)
    (Class|PixelStreamingInput|SendPixelStreamingResponse _pixelstreaminginput "{ \"Console\": \"r.setres 1920x1080w\" } or { \"Example_Event_01\": \"done\" }")))

(event EventBeginPlay
  (Utilities|FlowControl|Sequence
    (:then_0
      (Variables|Default|SetbShowMouseCursor true))
    (:then_1
      (Input|SetInputModeGameandUI self 0 "DoNotLock" true false))
    (:then_2)
    (:then_3)))

(fn ConstructionScript)

(fn Move&SeeLocationMinimap
  (params (LocationPoint :type Actor%20Object%20Reference))
  (bind _asbp_av_player (Utilities|Casting|CastToBp_AV_Player (Game|GetPlayerCharacter 0)))
  (Default|OrientMovement _asbp_av_player LocationPoint)
  (return))

(fn TouchRotation
  (params (Location_X :type Float%20%28double-precision%29) (Location_Y :type Float%20%28double-precision%29) (TouchRotation :type Float%20%28double-precision%29))
  (bind _returnvalue (Pawn|GetControlRotation :!class /Script/Engine.Controller))
  (bind _returnvalue_2 (* TouchRotation -1.0))
  (Variables|Default|SetTouch_Location_Current (Math|Vector2D|MakeVector2D Location_X Location_Y))
  (Pawn|SetControlRotation (Game|GetPlayerController 0) (Math|Rotator|MakeRotator 0.0 (Math|Float|ClampAngle (+ (.pitch _returnvalue) (* (* (- (/ (.y (Variables|Default|GetTouch_Location_Current)) (.y (Variables|Default|GetTouch_Location_Previous))) 1.0) -1.0) _returnvalue_2)) (Variables|Default|GetPitchLimit_Min) (Variables|Default|GetPitchLimit_Max)) (+ (* (- (/ (.x (Variables|Default|GetTouch_Location_Current)) (.x (Variables|Default|GetTouch_Location_Previous))) 1.0) _returnvalue_2) (.yaw _returnvalue))))
  (Variables|Default|SetTouch_Location_Previous (Math|Vector2D|MakeVector2D (.x (Variables|Default|GetTouch_Location_Current)) (.y (Variables|Default|GetTouch_Location_Current)))))

(fn SimpleMoveLocation
  (params (Location :type Vector) (Is%20Floor :type Boolean))
  (bind _returnvalue (Math|Vector|MakeVector (.x Location) (.y Location) 0.0))
  (if Is%20Floor
    (AI|Navigation|SimpleMovetoLocation self _returnvalue)
    (Game|SpawnActorfromClass "/Game/Blueprint/Character/Bp_TarguetPlayer.Bp_TarguetPlayer_C" (Math|Transform|MakeTransform _returnvalue "0, 0, 0" "1.000000,1.000000,1.000000") "Undefined" "OverrideRootScale" 0 0)
    (Development|PrintString "MOVE TO POINT")
    (return)
    (else
      (Development|PrintString "NO ES FLOOR"))))

(fn GetClickTouchLocation
  (bind (_worldlocation _worlddirection) (Game|Player|ConvertMouseLocationToWorldSpace))
  (bind _is_tactil (Variables|Default|GetIs_Tactil))
  (bind _location_x_screen (Variables|Default|GetLocation%20X_Screen))
  (bind _location_y_screen (Variables|Default|GetLocation%20Y_Screen))
  (bind (_worldlocation_2 _worlddirection_2) (Class|PlayerController|DeprojectScreenPositiontoWorld _location_x_screen _location_y_screen))
  (bind (_outhit _returnvalue) (Collision|LineTraceByChannel (Math|Vector|SelectVector _worldlocation_2 _worldlocation _is_tactil) (+ (Math|Vector|SelectVector _worldlocation_2 _worldlocation _is_tactil) (* (Math|Vector|SelectVector _worlddirection_2 _worlddirection _is_tactil) (Math|Conversions|ToVector(Float) 2.5e+03))) "TraceTypeQuery1" true 0 "ForDuration" true "(R=1.000000,G=0.000000,B=0.000000,A=1.000000)" "(R=0.000000,G=1.000000,B=0.000000,A=1.000000)" 3.0))
  (if _returnvalue
    (Development|PrintString "HIT")
    (Variables|Default|SetHit%20Actor (.HitActor (Collision|BreakHitResult _outhit)))
    (return (.Location (Collision|BreakHitResult _outhit)) (Actor|ActorHasTag (.HitActor (Collision|BreakHitResult _outhit)) "FLOOR"))
    (else
      (Development|PrintString "NO HIT - TOO FAR"))))