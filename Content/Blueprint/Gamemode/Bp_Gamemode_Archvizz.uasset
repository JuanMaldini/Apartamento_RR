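; Game mode for an archviz experience that sets up the UI and master sequence when play begins.
; It caches the archviz player controller, pre-creates widgets including HUD, minimap, pause, floorplan and controls, and creates a player for SEQ_Master.
; Outside floorplan mode, it shows either the controls or HUD widget after a short delay, chosen by the controller's MakeSEQ flag.
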(event EventBeginPlay
  (Utilities|FlowControl|Sequence
    (:then_0
      (bind _asbp_controller_archvizz (Utilities|Casting|CastToBp_Controller_Archvizz (Game|GetPlayerController 0)))
      (Variables|Default|SetAs%20Bp%20Controller%20Archvizz _asbp_controller_archvizz))
    (:then_1
      (bind _returnvalue (UserInterface|CreateWidget "/Game/UIMaterialLab/Widgets/W_HUD.W_HUD_C"))
      (Variables|Default|SetW_HUD _returnvalue))
    (:then_2
      (bind _returnvalue_2 (UserInterface|CreateWidget "/Game/UIMaterialLab/Widgets/W_Minimap.W_Minimap_C"))
      (Variables|Default|SetW_Minimap _returnvalue_2))
    (:then_3
      (bind _returnvalue_3 (UserInterface|CreateWidget "/Game/UIMaterialLab/Widgets/W_Pause.W_Pause_C"))
      (Variables|Default|SetW_Pause _returnvalue_3))
    (:then_4
      (bind _returnvalue_4 (UserInterface|CreateWidget "/Game/UIMaterialLab/Widgets/W_Credits.W_Credits_C"))
      (Variables|Default|SetW_Credits _returnvalue_4))
    (:then_5
      (bind _returnvalue_5 (UserInterface|CreateWidget "/Game/UIMaterialLab/Widgets/W_Layout.W_Layout_C"))
      (Variables|Default|SetW_Layout _returnvalue_5))
    (:then_6
      (bind _returnvalue_6 (UserInterface|CreateWidget "/Game/UIMaterialLab/Widgets/W_Cinematics.W_Cinematics_C"))
      (Variables|Default|SetW_Cinematics _returnvalue_6))
    (:then_7
      (bind _returnvalue_7 (Sequencer|Player|CreateLevelSequencePlayer "/Game/Cinematics/SEQ_Master.SEQ_Master"))
      (Variables|Default|SetSEQ_Master _returnvalue_7))
    (:then_8
      (bind _returnvalue_8 (UserInterface|CreateWidget "/Game/UIMaterialLab/Widgets/W_Floorplan.W_Floorplan_C"))
      (Variables|Default|SetW_Floorplan _returnvalue_8))
    (:then_9
      (if (not (Variables|/Game/Blueprint/Gamemode/Bp_Controller_Archvizz.Bp_Controller_Archvizz_C|GetAs%20Floorplan (Variables|Default|GetAs%20Bp%20Controller%20Archvizz)))
        (if (Variables|/Game/Blueprint/Gamemode/Bp_Controller_Archvizz.Bp_Controller_Archvizz_C|GetMakeSEQ (Variables|Default|GetAs%20Bp%20Controller%20Archvizz))
          (Utilities|FlowControl|Delay 2.0)
          (UserInterface|Viewport|AddtoViewport (Variables|Default|GetW_Controls) 0)
          (else
            (Utilities|FlowControl|Delay 2.0)
            (UserInterface|Viewport|AddtoViewport (Variables|Default|GetW_HUD) 0)))))
    (:then_10
      (bind _returnvalue_9 (UserInterface|CreateWidget "/Game/UIMaterialLab/Widgets/W_Controls.W_Controls_C"))
      (Variables|Default|SetW_Controls _returnvalue_9))))

(fn ConstructionScript)