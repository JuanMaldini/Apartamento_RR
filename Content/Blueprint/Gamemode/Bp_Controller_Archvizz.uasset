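; Player controller for an archviz apartment presentation: startup sets console tweaks, project label, camera fade, mouse input, minimap and optional intro sequence.
; MakeFloorplan switches possession between the walkthrough character and a spawned explorer pawn with blocking volume, blending views.
; Floorplan mode hides StaticMeshActors tagged FLOORPLAN and can add the game mode's floorplan widget.
; It also handles high-res screenshots, level restarts, and Pixel Streaming input executed as console commands.
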(event Custom|RestartLevel01
  ;[0 0 0] RESTART LEVEL
  (Development|PrintString "Restart Level")
  (Utilities|FlowControl|Delay 1.0)
  (bind _returnvalue (Game|GetCurrentLevelName true))
  (Game|OpenLevel(byName) (Utilities|String|StringToName _returnvalue)))

(event Custom|RequestIntroSEQ
  (params (Condition :type Boolean))
  ;[0 0 0] MAKE CINEMATICS
  (if Condition
    (Utilities|FlowControl|Sequence
      (:then_0
        (Class|MovieSceneSequencePlayer|PlayLooping (Variables|/Game/Blueprint/Gamemode/Bp_Gamemode_Archvizz.Bp_Gamemode_Archvizz_C|GetSEQ_Master (Variables|Default|GetAs%20Bp%20Gamemode%20Archvizz)) -1))
      (:then_1
        (UserInterface|Viewport|AddtoViewport (Variables|/Game/Blueprint/Gamemode/Bp_Gamemode_Archvizz.Bp_Gamemode_Archvizz_C|GetW_Cinematics (Variables|Default|GetAs%20Bp%20Gamemode%20Archvizz)) 0)))
    (else
      (Class|MovieSceneSequencePlayer|GotoEndandStop (Variables|/Game/Blueprint/Gamemode/Bp_Gamemode_Archvizz.Bp_Gamemode_Archvizz_C|GetSEQ_Master (Variables|Default|GetAs%20Bp%20Gamemode%20Archvizz))))))

(event Custom|PixelInput
  (params (Descriptor :type String))
  (bind _pixelstreaminginput (Variables|Components|GetPixelStreamingInput))
  (Variables|Default|SetDescriptor Descriptor)
  (if (.Success (Class|PixelStreamingInput|GetJsonStringValue _pixelstreaminginput (Variables|Default|GetDescriptor)))
    (Development|ExecuteConsoleCommand (.StringValue (Class|PixelStreamingInput|GetJsonStringValue _pixelstreaminginput (Variables|Default|GetDescriptor))) 0)
    (Class|PixelStreamingInput|SendPixelStreamingResponse _pixelstreaminginput "{ \"Console\": \"r.setres 1920x1080w\" } or { \"Example_Event_01\": \"done\" }")))

(event Custom|MakeFloorplan
  (params (bFloorplan :type Boolean) (AddWidget :type Boolean) (CanClick :type Boolean))
  (bind _as_bp_av_player (Variables|Default|GetAs%20Bp%20AV%20Player))
  (bind _as_bp_av_player_2 (Variables|Default|GetAs%20Bp%20AV%20Player))
  ;[0 0 0] MAKE FLOORPLAN
  (Utilities|FlowControl|Sequence
    (:then_0
      (if bFloorplan
        (CallFunction|FloorplanObjects true)
        (bind _returnvalue (Game|SpawnActorfromClass "/Game/Blueprint/ArchVizExplorer/BP_Explorer_Pawn.BP_Explorer_Pawn_C" (Math|Transform|MakeTransform "0.000000,0.000000,50.000000" "0, 0, 0" "1.000000,1.000000,1.000000") "Undefined" "MultiplyWithRoot" 0 0))
        (bind _output_get (Variables|Default|SetBP_Explorer_Pawn _returnvalue))
        (Game|Player|SetViewTargetwithBlend _output_get 0.5 "VTBlend_Linear" 0.0 false)
        (Utilities|FlowControl|Delay 0.5)
        (Collision|SetActorEnableCollision _as_bp_av_player_2 false)
        (Pawn|UnPossess)
        (Pawn|Possess _output_get)
        (bind _returnvalue_2 (Game|SpawnActorfromClass "/Game/Blueprint/Bp_BlockingVolume.Bp_BlockingVolume_C" (Math|Transform|MakeTransform "0, 0, 0" "0, 0, 0" "1.000000,1.000000,1.000000") "Undefined" "MultiplyWithRoot" 0 0))
        (Variables|Default|SetBp_Collision _returnvalue_2)
        (Variables|Default|SetPlayer_W_Location (Transformation|GetWorldTransform (Variables|/Script/Engine.Character|GetCapsuleComponent (Variables|Default|GetAs%20Bp%20AV%20Player))))
        (else
          (CallFunction|FloorplanObjects false)
          (Game|Player|SetViewTargetwithBlend _as_bp_av_player 0.5 "VTBlend_Linear" 0.0 false)
          (Utilities|FlowControl|Delay 0.5)
          (Pawn|UnPossess)
          (Collision|SetActorEnableCollision _as_bp_av_player_2 true)
          (Pawn|Possess _as_bp_av_player)
          (Actor|DestroyActor (Variables|Default|GetBP_Explorer_Pawn))
          (Actor|DestroyActor (Variables|Default|GetBp_Collision)))))
    (:then_1
      (Variables|Default|SetAs%20Floorplan bFloorplan))
    (:then_2
      (|AddWidgetToViewport AddWidget))
    (:then_3
      (Variables|Default|SetCanClick CanClick))))

(event EventBeginPlay
  (bind _returnvalue (Game|GetPlayerCameraManager 0))
  (bind _makeseq (Variables|Default|GetMakeSEQ))
  (Utilities|FlowControl|Sequence
    (:then_0
      (Development|ExecuteConsoleCommand "DumpUnbuiltLightInteractions" 0)
      (Development|ExecuteConsoleCommand "t.MaxFPS 5000" 0)
      (Development|ExecuteConsoleCommand "r.Streaming.PoolSize 20000" 0))
    (:then_1
      (CallFunction|FloorplanObjects false))
    (:then_2
      (bind _asbp_player_archvizz (Utilities|Casting|CastToBp_Player_Archvizz (Game|GetPlayerCharacter 0)))
      (Variables|Default|SetAs%20Bp%20AV%20Player _asbp_player_archvizz))
    (:then_3
      (bind _asbp_gamemode_archvizz (Utilities|Casting|CastToBp_Gamemode_Archvizz (Game|GetGameMode)))
      (Variables|Default|SetAs%20Bp%20Gamemode%20Archvizz _asbp_gamemode_archvizz))
    (:then_4
      ;[0 0 0] BOTTOM RIGHT TEXT
      (Variables|Default|SetProjectNameText (Utilities|Text|MakeLiteralText "Apartamento RR / Nati Minas & Studio + Flipê Arquitetura"))
      (Variables|Default|SetProjectNameSizeText 15))
    (:then_5
      (Class|PlayerCameraManager|SetManualCameraFade :self _returnvalue :InFadeAmount 1.0)
      (Utilities|FlowControl|Delay 1.0)
      (CameraFades|StartCameraFade :self _returnvalue :FromAlpha 1.0 :Duration 1.0 :bHoldWhenFinished true))
    (:then_6
      (if (Variables|Default|GetAs%20Floorplan)
        (CallFunction|MakeFloorplan true true false))
      (CallFunction|RequestIntroSEQ _makeseq)
      (Variables|Default|SetCanClick (not _makeseq)))
    (:then_7
      (Game|SpawnActorfromClass "/Game/Blueprint/Minimap/BP_Minimap.Bp_Minimap_C" (Math|Transform|MakeTransform "0, 0, 0") "Undefined" "MultiplyWithRoot" 0 0))
    (:then_8
      (Variables|Default|SetbShowMouseCursor true))
    (:then_9
      (Input|SetInputModeGameandUI self 0 "DoNotLock" true false))
    (:then_10)
    (:then_11
      (EventDispatchers|BindEventtoOnInputEvent (Variables|Components|GetPixelStreamingInput) (delegate Custom|PixelInput)))))

(event Input|ActionEvents|InputActionRestartLevel
  (params (Key :type Key%20Structure :default "None"))
  ;[0 0 0] RESTART LEVEL
  (:Pressed
    (Development|PrintString "Restart Level")
    (Utilities|FlowControl|Delay 1.0)
    (bind _returnvalue (Game|GetCurrentLevelName true))
    (Game|OpenLevel(byName) (Utilities|String|StringToName _returnvalue))))

(event Input|KeyboardEvents|P
  (params (Key :type Key%20Structure :default "None"))
  (bind _returnvalue (Viewport|GetViewportSize))
  ;[0 0 0] SCREENSHOT
  (:Pressed
    (Class|AutomationBlueprintFunctionLibrary|TakeHighResScreenshot (Math|Float|Truncate (.x _returnvalue)) (Math|Float|Truncate (.y _returnvalue)) "" 0 false false "Low" "" 0.0)))

(fn ConstructionScript)

(fn FloorplanObjects
  (params (bIsFloorplan :type Boolean))
  (if bIsFloorplan
    (Utilities|FlowControl|Sequence
      (:then_0
        (bind _outactors (Actor|GetAllActorsOfClass "/Script/Engine.StaticMeshActor"))
        (for _array_element _outactors
          (if (Actor|ActorHasTag _array_element "FLOORPLAN")
            (Rendering|SetActorHiddenInGame _array_element true))))
      (:then_1
        (return)))
    (else
      (Utilities|FlowControl|Sequence
        (:then_0
          (bind _outactors_2 (Actor|GetAllActorsOfClass "/Script/Engine.StaticMeshActor"))
          (for _array_element_2 _outactors_2
            (if (Actor|ActorHasTag _array_element_2 "FLOORPLAN")
              (Rendering|SetActorHiddenInGame _array_element_2 false))))
        (:then_1
          (return))))))