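; Player controller for point-and-click navigation by mouse or touch, which also spawns the minimap and handles level restart.
; Both inputs share a Visibility trace from screen position and a retriggerable-delay click check: double moves to FLOOR-tagged points with a target marker, single calls Interact on the hit Bp_Interact.
; Touch drag rotates the view with clamped pitch.
; A Pixel Streaming console-command handler exists, but its binding is unconnected.
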(event Custom|PixelInput
  (params (Descriptor :type String))
  (bind _pixelstreaminginput (Variables|Default|GetPixelStreamingInput))
  (Variables|Default|SetDescriptor Descriptor)
  (if (.Success (Class|PixelStreamingInput|GetJsonStringValue _pixelstreaminginput (Variables|Default|GetDescriptor)))
    (Development|ExecuteConsoleCommand (.StringValue (Class|PixelStreamingInput|GetJsonStringValue _pixelstreaminginput (Variables|Default|GetDescriptor))) 0)
    (Class|PixelStreamingInput|SendPixelStreamingResponse _pixelstreaminginput "{ \"Console\": \"r.setres 1920x1080w\" } or { \"Example_Event_01\": \"done\" }")))

(event EventBeginPlay
  (Utilities|FlowControl|Sequence
    (:then_0
      (Game|SpawnActorfromClass "/Game/Blueprint/Minimap/BP_Minimap.Bp_Minimap_C" (Math|Transform|MakeTransform "0, 0, 0") "Undefined" "MultiplyWithRoot" 0 0))
    (:then_1
      (Input|SetInputModeGameandUI self 0 "DoNotLock" true false))
    (:then_3)
    (:then_4)))

(event Input|ActionEvents|InputActionSetDestinationTarget
  (params (Key :type Key%20Structure))
  (:Pressed
    (Variables|Default|SetbShowMouseCursor true)
    (Variables|Default|SetIs_Tactil false)
    (Utilities|DoubleClick
      (:Double
        (bind (_location _is_floor) (CallFunction|GetClickTouchLocation))
        (CallFunction|SimpleMoveLocation _location _is_floor))
      (:Simple
        (bind _hit_actor (CallFunction|GetClickTouchLocation))
        (bind _outactors (Actor|GetAllActorsOfClass "/Game/Blueprint/Interact/Bp_Interact.Bp_Interact_C"))
        (for _array_element _outactors
          (if (== (Variables|/Game/Blueprint/Interact/Bp_Interact.Bp_Interact_C|GetObject%20Reference _array_element) _hit_actor)
            (bind _asbp_interact (Utilities|Casting|CastToBp_Interact _array_element))
            (Default|Interact _asbp_interact)))))))

(event Input|ActionEvents|InputActionRestartLevel
  (params (Key :type Key%20Structure))
  ;[0 0 0] Restart Level
  (:Pressed
    (Development|PrintString "Restart Level")
    (Utilities|FlowControl|Delay 1.0)
    (bind _returnvalue (Game|GetCurrentLevelName true))
    (Game|OpenLevel(byName) (Utilities|String|StringToName _returnvalue))))

(event Input|TouchEvents|InputTouch
  (params (Location :type Vector) (FingerIndex :type ETouchIndex%20Enum))
  (bind (_locationx _locationy _biscurrentlypressed) (Class|PlayerController|GetInputTouchState "Touch1"))
  (:Pressed
    (Variables|Default|SetLocation%20Y_Screen (.y Location))
    (Variables|Default|SetLocation%20X_Screen (.x Location))
    (Utilities|FlowControl|Sequence
      (:then_0
        (Variables|Default|SetbShowMouseCursor false)
        (Variables|Default|SetIs_Tactil true)
        (Utilities|DoubleClick
          (:Double
            (bind (_location _is_floor) (CallFunction|GetClickTouchLocation))
            (CallFunction|SimpleMoveLocation _location _is_floor))
          (:Simple
            (bind _hit_actor (CallFunction|GetClickTouchLocation))
            (bind _outactors (Actor|GetAllActorsOfClass "/Game/Blueprint/Interact/Bp_Interact.Bp_Interact_C"))
            (for _array_element _outactors
              (if (== (Variables|/Game/Blueprint/Interact/Bp_Interact.Bp_Interact_C|GetObject%20Reference _array_element) _hit_actor)
                (bind _asbp_interact (Utilities|Casting|CastToBp_Interact _array_element))
                (Default|Interact _asbp_interact))))))
      (:then_1
        (Variables|Default|SetTouch_Hold true)
        (Variables|Default|SetTouch_Location_Previous (Math|Vector2D|MakeVector2D _locationx _locationy) :!label _label))))
  (:Released
    (Utilities|FlowControl|Sequence
      (:then_0
        (if (Variables|Default|GetTouch_Hold)
          (Variables|Default|SetTouch_Hold false)))
      (:then_1
        (goto _label))))
  (:Moved
    (Variables|Default|SetLocation%20Y_Screen (.y Location))
    (Variables|Default|SetLocation%20X_Screen (.x Location))
    (if _biscurrentlypressed
      (CallFunction|TouchRotation _locationx _locationy 75.0))))

(fn ConstructionScript)

(fn Move&SeeLocationMinimap
  (params (LocationPoint :type Actor%20Object%20Reference))
  (bind _asbp_av_player (Utilities|Casting|CastToBp_AV_Player (Game|GetPlayerCharacter 0)))
  (Default|OrientMovement _asbp_av_player LocationPoint)
  (return))

(fn TouchRotation
  (params (Location_X :type Float%20%28double-precision%29) (Location_Y :type Float%20%28double-precision%29) (TouchRotation :type Float%20%28double-precision%29))
  (bind _returnvalue (Pawn|GetControlRotation :!class /Script/Engine.Controller))
  (bind _returnvalue_2 (* TouchRotation -1.0))
  (Variables|Default|SetTouch_Location_Current (Math|Vector2D|MakeVector2D Location_X Location_Y))
  (Pawn|SetControlRotation (Game|GetPlayerController 0) (Math|Rotator|MakeRotator 0.0 (Math|Float|ClampAngle (+ (.pitch _returnvalue) (* (* (- (/ (.y (Variables|Default|GetTouch_Location_Current)) (.y (Variables|Default|GetTouch_Location_Previous))) 1.0) -1.0) _returnvalue_2)) (Variables|Default|GetPitchLimit_Min) (Variables|Default|GetPitchLimit_Max)) (+ (* (- (/ (.x (Variables|Default|GetTouch_Location_Current)) (.x (Variables|Default|GetTouch_Location_Previous))) 1.0) _returnvalue_2) (.yaw _returnvalue))))
  (Variables|Default|SetTouch_Location_Previous (Math|Vector2D|MakeVector2D (.x (Variables|Default|GetTouch_Location_Current)) (.y (Variables|Default|GetTouch_Location_Current)))))

(fn CheckTargetDistance
  (params (Location%20Point :type Actor%20Object%20Reference) (Closer%20Min :type Float%20%28double-precision%29))
  (bind _asbp_av_player (Utilities|Casting|CastToBp_AV_Player (Game|GetPlayerCharacter 0)))
  (return (<= (Math|Vector|VectorLength (- (Transformation|GetActorLocation Location%20Point) (Transformation|GetActorLocation _asbp_av_player))) Closer%20Min)))

(fn SimpleMoveLocation
  (params (Location :type Vector) (Is%20Floor :type Boolean))
  (bind _returnvalue (Math|Vector|MakeVector (.x Location) (.y Location) 0.0))
  (if Is%20Floor
    (AI|Navigation|SimpleMovetoLocation self _returnvalue)
    (Game|SpawnActorfromClass "/Game/Blueprint/Character/Bp_TarguetPlayer.Bp_TarguetPlayer_C" (Math|Transform|MakeTransform _returnvalue "0, 0, 0" "1.000000,1.000000,1.000000") "Undefined" "OverrideRootScale" 0 0)
    (Development|PrintString "MOVE TO POINT")
    (return)
    (else
      (Development|PrintString "NO ES FLOOR"))))

(fn GetClickTouchLocation
  (bind (_worldlocation _worlddirection) (Game|Player|ConvertMouseLocationToWorldSpace))
  (bind _is_tactil (Variables|Default|GetIs_Tactil))
  (bind _location_x_screen (Variables|Default|GetLocation%20X_Screen))
  (bind _location_y_screen (Variables|Default|GetLocation%20Y_Screen))
  (bind (_worldlocation_2 _worlddirection_2) (Class|PlayerController|DeprojectScreenPositiontoWorld _location_x_screen _location_y_screen))
  (bind (_outhit _returnvalue) (Collision|LineTraceByChannel (Math|Vector|SelectVector _worldlocation_2 _worldlocation _is_tactil) (+ (Math|Vector|SelectVector _worldlocation_2 _worldlocation _is_tactil) (* (Math|Vector|SelectVector _worlddirection_2 _worlddirection _is_tactil) (Math|Conversions|ToVector(Float) 2.5e+03))) "TraceTypeQuery1" true 0 "ForDuration" true "(R=1.000000,G=0.000000,B=0.000000,A=1.000000)" "(R=0.000000,G=1.000000,B=0.000000,A=1.000000)" 3.0))
  (if _returnvalue
    (Development|PrintString "HIT")
    (bind _output_get (Variables|Default|SetHit%20Actor (.HitActor (Collision|BreakHitResult _outhit))))
    (return (.Location (Collision|BreakHitResult _outhit)) (Actor|ActorHasTag (.HitActor (Collision|BreakHitResult _outhit)) "FLOOR") _output_get)
    (else
      (Development|PrintString "NO HIT - TOO FAR"))))