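; Intro sequence controller for an archviz level that starts and stops the SEQ_Master cinematic.
; BeginPlay creates and stores a level sequence player.
; MakeSEQ fetches the cinematics widget from Bp_Gamemode_Archvizz, then either loops the sequence indefinitely and adds the widget to the viewport, or jumps to the end and stops.
; The stop branch leaves the widget untouched.
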(event EventBeginPlay
  (bind _returnvalue (Sequencer|Player|CreateLevelSequencePlayer "/Game/Cinematics/SEQ_Master.SEQ_Master"))
  (Variables|Default|SetSEQ_Master _returnvalue))

(fn ConstructionScript)

(fn MakeSEQ
  (params (Condition :type Boolean))
  (bind _seq_master (Variables|Default|GetSEQ_Master))
  (Utilities|FlowControl|Sequence
    (:then_0
      (bind _asbp_gamemode_archvizz (Utilities|Casting|CastToBp_Gamemode_Archvizz (Game|GetGameMode)))
      (Variables|Default|SetW%20Cinematics (Variables|/Game/Blueprint/Gamemode/Bp_Gamemode_Archvizz.Bp_Gamemode_Archvizz_C|GetW_Cinematics _asbp_gamemode_archvizz)))
    (:then_1
      (if Condition
        (Class|MovieSceneSequencePlayer|PlayLooping _seq_master -1)
        (UserInterface|Viewport|AddtoViewport (Variables|Default|GetW%20Cinematics) 0)
        (else
          (Class|MovieSceneSequencePlayer|GotoEndandStop _seq_master))))))